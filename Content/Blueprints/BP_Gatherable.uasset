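; BP_Gatherable is a gatherable item Blueprint with an InteractUI widget that shows a WBP_Interactable.
; On BeginPlay it assigns its Item to that widget's InteractItem.
; When OnItemDroppedBP fires, it replaces InteractItem with the dropped item and prints a debug string.
; The Blueprint only feeds the widget; it contains no gathering logic of its own.
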(event EventBeginPlay
  (bind _aswbp_interactable (Utilities|Casting|CastToWBP_Interactable (UserInterface|GetUserWidgetObject (Variables|Default|GetInteractUI))))
  (Variables|/Game/UI/WBP_Interactable.WBP_Interactable_C|SetInteractItem _aswbp_interactable (Variables|Default|GetItem)))

(event EventOnItemDroppedBP
  (params (DroppedItem :type Item%20Object%20Reference))
  (bind _aswbp_interactable (Utilities|Casting|CastToWBP_Interactable (UserInterface|GetUserWidgetObject (Variables|Default|GetInteractUI))))
  (Variables|/Game/UI/WBP_Interactable.WBP_Interactable_C|SetInteractItem _aswbp_interactable DroppedItem)
  (Development|PrintString "DROPPPP"))

(fn ConstructionScript)