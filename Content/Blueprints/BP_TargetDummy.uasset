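; BP_TargetDummy is a target dummy that displays the damage it takes on a widget.
; On BeginPlay it casts its widget component's user widget to WBP_TargetDummy, caches the TargetDamage text and sets itself as the widget's OwningCharacter.
; HandleTakeAnyDamageBP overwrites that text with each incoming damage value truncated to an integer, so it shows the latest hit rather than a running total.
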(event EventBeginPlay
  (bind _aswbp_target_dummy (Utilities|Casting|CastToWBP_TargetDummy (UserInterface|GetUserWidgetObject (Variables|Default|GetWidget))))
  (Variables|Default|SetTargetDMG (Variables|/Game/UI/WBP_TargetDummy.WBP_TargetDummy_C|GetTargetDamage _aswbp_target_dummy))
  (Variables|/Game/UI/WBP_TargetDummy.WBP_TargetDummy_C|SetOwningCharacter _aswbp_target_dummy self))

(event EventHandleTakeAnyDamageBP
  (params (DamagedActor :type Actor%20Object%20Reference) (Damage :type Float%20%28single-precision%29) (DamageType :type Damage%20Type%20Object%20Reference) (InstigatedBy :type Controller%20Object%20Reference) (DamageCauser :type Actor%20Object%20Reference))
  (Rendering|Components|TextRender|SetText (Variables|Default|GetTargetDMG) (Utilities|Text|ToText(String) (Class|KismetMathLibrary|FTrunc64 Damage))))

(fn ConstructionScript)